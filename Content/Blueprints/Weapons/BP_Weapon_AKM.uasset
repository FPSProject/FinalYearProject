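; AKM rifle weapon that attaches to the Shooter's hands and deals hitscan damage.
; Equip attaches it at WeaponSocket and binds FireWeapon to the Shooter's fire dispatcher.
; FireWeapon runs a debug-drawn object trace along camera forward, starting from an offset off the muzzle socket.
; Damage applies only when the hit component's object type is GameTraceChannel1, which is absent from the traced types.
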(event Custom|FireWeapon
  ;[1 1 1] Line Trace for object
  (bind (_start _end) (CallFunction|GetLineTraceLocation (Variables|/Game/Blueprints/Characters/Shooter.Shooter_C|GetCamera (stale Custom|Equip _asshooter)) (Transformation|GetSocketLocation (Variables|Default|GetAMK) "BulletPointSocket")))
  (bind (_outhit _returnvalue) (Collision|LineTraceForObjects _start _end (Utilities|Array|MakeArray "ObjectTypeQuery1" "ObjectTypeQuery2" "ObjectTypeQuery3" "ObjectTypeQuery4") false 0 "ForDuration"))
  (if _returnvalue
    (if (Utilities|Enum|Equal(Enum) (Collision|GetCollisionObjectType (.HitComponent (Collision|BreakHitResult _outhit))) "ECC_GameTraceChannel1")
      (Game|Damage|ApplyDamage (Components|GetOwner (.HitComponent (Collision|BreakHitResult _outhit))) (Variables|Default|GetbaseDamage) 0 0))))

(event Custom|Equip
  (params (ShooterUser :type Actor%20Object%20Reference))
  ;[1 1 1] Attach Weapon to player
  (bind _asshooter (Utilities|Casting|CastToShooter ShooterUser)
    (:then
      (Development|PrintString "Succeeded Cast")
      (Transformation|AttachComponentToComponent (Variables|/Game/Blueprints/Characters/Shooter.Shooter_C|GetHands _asshooter) "WeaponSocket" "KeepRelative" "KeepRelative" "KeepRelative" true)
      (EventDispatchers|BindEventtoFireWeaponDispatch _asshooter (delegate Custom|FireWeapon)))
    (:CastFailed
      (CallFunction|ErrorMessage "Cast to shooter failed -> BP_Weapon_AKM"))))

(fn ConstructionScript)

(fn ErrorMessage
  (params (InString :type String))
  (Development|PrintString InString true true "(R=1.000000,G=0.000000,B=0.000000,A=1.000000)" 5.0))

(fn GetLineTraceLocation
  (params (CamComp :type Camera%20Component%20Object%20Reference) (socketLocation :type Vector))
  (bind _returnvalue (Transformation|GetWorldRotation CamComp))
  (bind _returnvalue_2 (Math|Vector|RotateVector "100.000000,0.000000,-10.000000" _returnvalue))
  (bind _returnvalue_3 (+ socketLocation _returnvalue_2))
  (return _returnvalue_3 (+ (* (Math|Vector|GetForwardVector CamComp) 9999.0) _returnvalue_3)))