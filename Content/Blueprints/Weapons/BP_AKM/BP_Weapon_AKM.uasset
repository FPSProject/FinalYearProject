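; AKM weapon Blueprint that attaches to the Shooter's camera socket on Equip and binds to its fire dispatcher.
; Firing line-traces along the camera's forward vector from an offset off the muzzle socket.
; It spawns a BP_Projectile_AKM aimed at the impact point, or at the trace end on a miss.
; The trace itself applies damage, higher or lower by the hit component's custom collision object type.
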(event Custom|FireWeapon
  ;[1 1 1] Line Trace for object
  (bind (_start _end) (CallFunction|GetLineTraceLocation (Variables|/Game/Blueprints/Characters/Shooter.Shooter_C|GetCamera (stale Custom|Equip _asshooter)) (Transformation|GetSocketLocation (Variables|Default|GetSkeletalMesh) "ProjectileSocket")))
  (bind (_outhit _returnvalue) (Collision|LineTraceForObjects _start _end (Utilities|Array|MakeArray "ObjectTypeQuery7" "ObjectTypeQuery1" "ObjectTypeQuery8") false 0 "None"))
  (CallFunction|SpawnProjectile (.ImpactPoint (Collision|BreakHitResult _outhit)) (.TraceEnd (Collision|BreakHitResult _outhit)) _returnvalue)
  (if _returnvalue
    (if (Utilities|Enum|Equal(Enum) (Collision|GetCollisionObjectType (.HitComponent (Collision|BreakHitResult _outhit))) "ECC_GameTraceChannel1")
      (Variables|Default|SetbaseDamage 5e+01)
      (Game|Damage|ApplyDamage (Components|GetOwner (.HitComponent (Collision|BreakHitResult _outhit))) (Variables|Default|GetbaseDamage) 0 0 :!label _label)
      (Variables|Default|SetbaseDamage 0.0)
      (elif (Utilities|Enum|Equal(Enum) (Collision|GetCollisionObjectType (.HitComponent (Collision|BreakHitResult _outhit))) "ECC_GameTraceChannel2")
        (Variables|Default|SetbaseDamage 1e+01)
        (goto _label)))))

(event Custom|Equip
  (params (ShooterUser :type Actor%20Object%20Reference))
  ;[1 1 1] Attach Weapon to player
  (bind _asshooter (Utilities|Casting|CastToShooter ShooterUser)
    (:then
      (Development|PrintString "Succeeded Cast")
      (Transformation|AttachComponentToComponent (Variables|/Game/Blueprints/Characters/Shooter.Shooter_C|GetCamera _asshooter) "WeaponSocket" "SnapToTarget" "SnapToTarget" "SnapToTarget" true)
      (EventDispatchers|BindEventtoFireWeaponDispatch _asshooter (delegate Custom|FireWeapon)))
    (:CastFailed
      (CallFunction|ErrorMessage "Cast to shooter failed -> BP_Weapon_AKM"))))

(fn ConstructionScript)

(fn ErrorMessage
  (params (InString :type String))
  (Development|PrintString InString true true "(R=1.000000,G=0.000000,B=0.000000,A=1.000000)" 5.0))

(fn GetLineTraceLocation
  (params (CamComp :type Camera%20Component%20Object%20Reference) (socketLocation :type Vector))
  (bind _returnvalue (Transformation|GetWorldRotation CamComp))
  (bind _returnvalue_2 (Math|Vector|RotateVector "100.000000,0.000000,-10.000000" _returnvalue))
  (bind _returnvalue_3 (+ socketLocation _returnvalue_2))
  (return _returnvalue_3 (+ (* (Math|Vector|GetForwardVector CamComp) 999999.0) _returnvalue_3)))

(fn SpawnProjectile
  (params (A :type Vector) (B :type Vector) (bPickA :type Boolean))
  (bind _skeletalmesh (Variables|Default|GetSkeletalMesh))
  (bind _returnvalue (Transformation|GetSocketLocation _skeletalmesh "ProjectileSocket"))
  (Game|SpawnActorfromClass "/Game/Blueprints/Projectiles/BP_Projectile_AKM.BP_Projectile_AKM_C" (Math|Transform|MakeTransform _returnvalue (Math|Rotator|FindLookatRotation _returnvalue (Math|Vector|SelectVector A B bPickA))) "Undefined" 0 0))